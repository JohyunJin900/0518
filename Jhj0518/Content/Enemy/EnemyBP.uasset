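; Enemy actor Blueprint with its own health that deals repeated damage to an overlapping hero.
; An overlapping actor that implements DamageInterface is stored as Hero, starting a looping timer that sends it DecreaseHpMessage with fixed damage.
; The timer is cleared when that Hero leaves the overlap.
; A custom event subtracts incoming damage from Hp and destroys the enemy at zero or below.
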(event `self.ReceiveBeginPlay`
  (set `self.Hp` 100.0))

(event `CustomEvent`
  (params (Amount :type "Float (double-precision)"))
  (bind _output_get (set `self.Hp` (- (`self.Hp`) Amount)))
  (if (<= _output_get 0.0)
    (`self.K2_DestroyActor`)))

(event `self.ReceiveActorBeginOverlap`
  (params (OtherActor :type "Actor Object Reference"))
  (if (`KismetSystemLibrary.DoesImplementInterface` OtherActor "/Game/Interface/DamageInterface.DamageInterface_C")
    (set `self.Hero` OtherActor)
    (`KismetSystemLibrary.K2_SetTimer` null "DecreaseHeroHP" 0.33 true)))

(event `DecreaseHeroHP`
  (message `/Game/Interface/DamageInterface.DecreaseHp` (`self.Hero`) 30.0))

(event `self.ReceiveActorEndOverlap`
  (params (OtherActor :type "Actor Object Reference"))
  (if (== OtherActor (`self.Hero`))
    (`KismetSystemLibrary.K2_ClearTimer` null "DecreaseHeroHP")))

(fn `UserConstructionScript`)