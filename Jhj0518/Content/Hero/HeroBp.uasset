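; Player hero Blueprint that moves, turns, fires a gun and tracks health.
; BeginPlay sets starting HP, spawns a GunBP and snaps it to the mesh's GunPoint socket; the TriggerBullet input starts and stops its firing.
; Movement axes push along fixed world X and Y regardless of facing, while Turn rotates the actor's yaw.
; DecreaseHp subtracts damage, prints remaining HP and destroys the hero at zero or below.
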(event `/Game/Interface/DamageInterface.DecreaseHp`
  (params (Amount :type "Float (single-precision)"))
  (bind _hp (`self.Hp`))
  (bind _output_get (set `self.Hp` (- _hp Amount)))
  (`KismetSystemLibrary.PrintString` (`KismetStringLibrary.Conv_DoubleToString` _hp))
  (if (<= _output_get 0.0)
    (`self.K2_DestroyActor`)))

(event `InputAction|TriggerBullet`
  (params (Key :type "Key Structure" :default "AnyKey"))
  (bind _gun (`self.Gun`))
  (:`Pressed`
    (`/Game/Gun/GunBP.StartFiring` _gun))
  (:`Released`
    (`/Game/Gun/GunBP.StopFiring` _gun)))

(event `self.ReceiveBeginPlay`
  (set `self.Hp` 100.0)
  (bind _returnvalue (`|SpawnActorFromClass` "/Game/Gun/GunBP.GunBP_C" (`SceneComponent.K2_GetComponentToWorld` (`self.Mesh`)) "Undefined" "OverrideRootScale"))
  (bind _output_get (set `self.Gun` _returnvalue))
  (`self.K2_AttachToComponent` _output_get (`self.Mesh`) "GunPoint" "SnapToTarget" "SnapToTarget" "KeepRelative" true))

(event `InputAxis|MoveForward`
  (params (AxisValue :type "Float (single-precision)"))
  (`self.AddMovementInput` (1.0 0.0 0.0) AxisValue))

(event `InputAxis|MoveRight`
  (params (AxisValue :type "Float (single-precision)"))
  (`self.AddMovementInput` (0.0 1.0 0.0) AxisValue))

(event `InputAxis|Turn`
  (params (AxisValue :type "Float (single-precision)"))
  (`self.K2_AddActorLocalRotation` (`KismetMathLibrary.MakeRotator` 0.0 0.0 (* AxisValue 3.0))))

(fn `UserConstructionScript`)